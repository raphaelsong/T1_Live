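; Monster character with melee attacks, a health bar and a death that reports a positive game result.
; Attack sets the anim-blueprint flag and halts movement until a one-second timer restores both; AttackHitCheck sphere-traces forward and deals damage through T1CombatComponent.
; BeginPlay binds HP-change and zero-HP events on that component and initializes the widget bar.
; SetDead plays the death montage, disables collision, hides the bar, stops AI and notifies the GameMode.
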(event `self.ReceiveBeginPlay`
  (add `/Game/Blueprints/Components/T1CombatComponent.OnChangedHp` (`self.T1CombatComponent`) (`|CreateDelegate` :!event `UpdateHp`))
  (`self.UpdateHp` (`/Game/Blueprints/Components/T1CombatComponent.Hp` (`self.T1CombatComponent`)) (`/Game/Blueprints/Components/T1CombatComponent.MaxHp` (`self.T1CombatComponent`)))
  (add `/Game/Blueprints/Components/T1CombatComponent.OnHpZero` (`self.T1CombatComponent`) (`|CreateDelegate` :!event `SetDead`)))

(fn `Attack`
  (bind _asabp_t1monster (cast `/Game/Animation/ABP_T1Monster` (`SkeletalMeshComponent.GetAnimInstance` (`self.Mesh`))))
  (set `/Game/Animation/ABP_T1Monster.IsAttack` true _asabp_t1monster)
  (`CharacterMovementComponent.SetMovementMode` (`self.CharacterMovement`) "MOVE_None" 0)
  (`KismetSystemLibrary.K2_SetTimer` null "AttackEnded" 1.0))

(fn `AttackEnded`
  (bind _asabp_t1monster (cast `/Game/Animation/ABP_T1Monster` (`SkeletalMeshComponent.GetAnimInstance` (`self.Mesh`))))
  (set `/Game/Animation/ABP_T1Monster.IsAttack` false _asabp_t1monster)
  (`CharacterMovementComponent.SetMovementMode` (`self.CharacterMovement`) "MOVE_Walking" 0))

(fn `AttackHitCheck`
  (bind _returnvalue (`self.K2_GetActorLocation`))
  (bind (_outhit _returnvalue_2) (`KismetSystemLibrary.SphereTraceSingle` :`Start` _returnvalue :`End` (+ _returnvalue (* (`self.GetActorForwardVector`) (`self.AttackRange`))) :`Radius` (`self.AttackRadius`) :`TraceChannel` "TraceTypeQuery4" :`DrawDebugType` "ForDuration" :`DrawTime` 0.5))
  (if _returnvalue_2
    (`/Game/Blueprints/Components/T1CombatComponent.CombatAttack` (`self.T1CombatComponent`) (`self.DamageAmount`) (`.HitActor` (`GameplayStatics.BreakHitResult` _outhit)))))

(fn `SetDead`
  (`self.PlayAnimMontage` "/Game/Animation/AM_MonsterDeath.AM_MonsterDeath")
  (`self.SetActorEnableCollision` false)
  (`SceneComponent.SetHiddenInGame` (`self.HpBarWidget`) true false)
  (bind _asbp_t1aicontroller (cast `/Game/Blueprints/Controllers/BP_T1AIController` (`self.GetController`)))
  (`/Game/Blueprints/Controllers/BP_T1AIController.StopAI` _asbp_t1aicontroller)
  (`KismetSystemLibrary.K2_SetTimerDelegate` (`|CreateDelegate` :!event `K2_DestroyActor`) 5.0)
  (bind _asbp_t1game_mode (cast `/Game/Blueprints/GameModes/BP_T1GameMode` (`GameplayStatics.GetGameMode`)))
  (`/Game/Blueprints/GameModes/BP_T1GameMode.GameResult` _asbp_t1game_mode true))

(fn `UpdateHp`
  (params (InHp :type "Float (double-precision)") (InMaxHp :type "Float (double-precision)"))
  (bind _aswbp_hp_bar (cast `/Game/UI/WBP_HpBar` (`WidgetComponent.GetUserWidgetObject` (`self.HpBarWidget`))))
  (`/Game/UI/WBP_HpBar.UpdateHpBar` _aswbp_hp_bar InHp InMaxHp))

(fn `UserConstructionScript`)