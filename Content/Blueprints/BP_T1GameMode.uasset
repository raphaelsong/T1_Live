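; BP_T1GameMode is a game mode that handles the end of a match through its GameResult event.
; The event creates a WBP_GameResult widget, adds it to the viewport and passes it the success flag.
; On success it also spawns an actor at the player pawn's transform.
; Both outcomes pause the game after a short delay.
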(event `GameResult`
  (params (IsSuccess :type Boolean))
  (bind _returnvalue (`|CreateWidget` "/Game/UI/WBP_GameResult.WBP_GameResult_C"))
  (`UserWidget.AddToViewport` _returnvalue 0)
  (`/Game/UI/WBP_GameResult.SetResult` _returnvalue IsSuccess)
  (if IsSuccess
    (`|SpawnActorFromClass` "/Game/UI/BP_Congratulation.BP_Congratulation_C" (`self.GetTransform` (`GameplayStatics.GetPlayerPawn` 0)) "Undefined" "MultiplyWithRoot" null null)
    (`KismetSystemLibrary.Delay` 3.0)
    (`GameplayStatics.SetGamePaused` true)
    (else
      (`KismetSystemLibrary.Delay` 3.0)
      (`GameplayStatics.SetGamePaused` true))))

(fn `UserConstructionScript`)